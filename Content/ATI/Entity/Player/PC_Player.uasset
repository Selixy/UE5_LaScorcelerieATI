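; Player controller for the Bouloizeau game that routes the player's pause and exit inputs to the game mode.
; On BeginPlay it adds the IMC_Bouloizeau Enhanced Input mapping context and caches the cast BP_GameMode-Bouloizeau reference.
; The IA_Pause and IA_Exit Started events call Pause and Exit on that cached game mode, leaving the logic there.
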(event Input|EnhancedActionEvents|EnhancedInputActionIA_Pause
  (params (ActionValue :type Boolean) (ElapsedSeconds :type Float%20%28double-precision%29) (TriggeredSeconds :type Float%20%28double-precision%29) (InputAction :type Input%20Action%20Object%20Reference :default "/Game/ATI/Entity/Player/Input/Actions/IA_Pause.IA_Pause"))
  (:Started
    (Default|Pause (Variables|Default|GetGame%20Mode))))

(event Input|EnhancedActionEvents|EnhancedInputActionIA_Exit
  (params (ActionValue :type Boolean) (ElapsedSeconds :type Float%20%28double-precision%29) (TriggeredSeconds :type Float%20%28double-precision%29) (InputAction :type Input%20Action%20Object%20Reference :default "/Game/ATI/Entity/Player/Input/Actions/IA_Exit.IA_Exit"))
  (:Started
    (Default|Exit (Variables|Default|GetGame%20Mode))))

(event EventBeginPlay
  (|AddInputMapping)
  (bind _asbp_game_mode__bouloizeau (Utilities|Casting|CastToBP_GameMode-Bouloizeau (Game|GetGameMode)))
  (Variables|Default|SetGame%20Mode _asbp_game_mode__bouloizeau))

(event EventTick
  (params (DeltaSeconds :type Float%20%28single-precision%29)))

(fn ConstructionScript)