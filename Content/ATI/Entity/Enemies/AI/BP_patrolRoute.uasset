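; BP_patrolRoute is a spline-based patrol path for enemy AI.
; It tracks a current point index and exposes that spline point's world position through GetSplinePointAsWorldPosition.
; IncrementPatrolRoute steps the index along the spline and flips direction at the first and last points, producing a back-and-forth ping-pong route.
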(event Custom|IncrementPatrolRoute
  ;[0.8641 0.4034 0.9271] Déplacement le long de la curve
  (bind _output_get (Variables|Default|SetPatrolIndex (+ (Variables|Default|GetPatrolIndex) (Variables|Default|GetDirection))))
  ;[0.8262 0.2287 1] Verification que l'ennemi est arrivé au bout de la curvcurve et retour en arrière si c'est le cas
  (if (== _output_get (- (Spline|GetNumberOfSplinePoints (Variables|Default|GetPatrolRoute)) 1))
    (Variables|Default|SetDirection -1)
    (else
      ;[0.9363 0.5879 1] Cas contraire
      (if (== (Variables|Default|GetPatrolIndex) 0)
        (Variables|Default|SetDirection 1)))))

(fn ConstructionScript)

(fn GetSplinePointasWorldPosition
  ;[0.395 1 0.9701] Déplacement le long d'une curve en particulier
  (return (Spline|GetLocationatSplinePoint (Variables|Default|GetPatrolRoute) (Variables|Default|GetPatrolIndex) "World")))