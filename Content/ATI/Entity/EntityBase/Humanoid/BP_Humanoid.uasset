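; BP_Humanoid is a humanoid entity Blueprint that adds crouching and chargeable ability casting to its parent class.
; Crouch start and stop overrides switch the movement state enum.
; Ability events read DT_Ability rows: start spawns the charging Niagara effect, and the ongoing cast event applies stamina or mana charging costs and moves the effect to AimStart.
; The cast event passes charge time and aim to CastAbility, then destroys the effect.
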(event EventBeginPlay
  (|CallParentFunction))

(event Collision|EventActorBeginOverlap
  (params (OtherActor :type Actor%20Object%20Reference))
  (|CallParentFunction OtherActor))

(event EventTick
  (params (DeltaSeconds :type Float%20%28single-precision%29))
  (|CallParentFunction DeltaSeconds))

(event Custom|Parent%20:%20Stop%20Crouch
  (params (InputAction :type Input%20Action%20Object%20Reference))
  (Variables|MouvementSatue|SetMouvementState "NewEnumerator0"))

(event Custom|Parent%20:%20Start%20Crouch
  (params (InputAction :type Input%20Action%20Object%20Reference))
  (Variables|MouvementSatue|SetMouvementState "NewEnumerator1"))

(event Custom|CE_SartAbility
  (params (Ability :type Name))
  (bind _returnvalue (Utilities|GetDataTableRow "/Game/ATI/Entity/Ability/DT_Ability.DT_Ability" Ability)
    (:then
      (Variables|Default|SetSpelStruct _returnvalue)
      (Utilities|IsValid (Utilities|Struct|BreakS_VisuelAbility (Utilities|Struct|BreakS_Ability (Variables|Default|GetSpelStruct)))
        (:Is%20Valid
          (bind _returnvalue_2 (Class|NiagaraFunctionLibrary|SpawnSystematLocationwithParams (Utilities|Struct|MakeFXSystemSpawnParameters 0 (Utilities|Struct|BreakS_VisuelAbility (Utilities|Struct|BreakS_Ability (Variables|Default|GetSpelStruct))) (Transformation|GetWorldLocation (Variables|Default|GetAimStart)) "0.000000,0.000000,0.000000" "1.000000,1.000000,1.000000" 0 "None" "KeepWorldPosition" true true)))
          (Variables|Default|SetNiagaraCharging _returnvalue_2))))))

(event Custom|Parent%20:%20CE_CastAbility
  (params (ElapsedSec :type Float%20%28double-precision%29) (StartAndDirection :type S%20Double%20Vector%20Structure) (Ability :type Name))
  (CallFunction|CastAbility ElapsedSec StartAndDirection Ability self)
  (Components|DestroyComponent (Variables|Default|GetNiagaraCharging)))

(event Custom|Parent%20:%20CE_OnCastAbility
  (params (TrigeredSec :type Float%20%28double-precision%29) (Ability :type Name))
  (bind _returnvalue (Utilities|GetDataTableRow "/Game/ATI/Entity/Ability/DT_Ability.DT_Ability" Ability)
    (:then
      (Utilities|FlowControl|Sequence
        (:then_0
          (if (.Stamina? (Utilities|Struct|BreakS_CoutAbylity (Utilities|Struct|BreakS_Ability _returnvalue)))
            (CallFunction|AddStamina (Math|Conversions|ToFloat(Integer) (.StaminaChargingCost (Utilities|Struct|BreakS_CoutAbylity (Utilities|Struct|BreakS_Ability _returnvalue)))))))
        (:then_1
          (if (.Mana? (Utilities|Struct|BreakS_CoutAbylity (Utilities|Struct|BreakS_Ability _returnvalue)))
            (CallFunction|AddMana (Math|Conversions|ToFloat(Integer) (.ManaChargingCost (Utilities|Struct|BreakS_CoutAbylity (Utilities|Struct|BreakS_Ability _returnvalue)))))))
        (:then_2
          (Utilities|IsValid (Variables|Default|GetNiagaraCharging)
            (:Is%20Valid
              (Transformation|SetWorldLocation (Variables|Default|GetNiagaraCharging) (Transformation|GetWorldLocation (Variables|Default|GetAimStart)) false false))))))))

(fn ConstructionScript
  (|CallParentFunction))