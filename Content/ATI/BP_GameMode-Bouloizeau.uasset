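; Game mode Blueprint that handles pausing and sublevel resets.
; Pause toggles the gaming mode between in-game and paused, calls the pause event dispatcher, and shows or hides a lazily created pause menu widget.
; ResetLvl unloads a managed list of streaming sublevels, waits briefly, then reloads them visible.
; Helper functions add, set, remove or clear that list; the Exit event is empty.
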(event Custom|Pause
  (switch Utilities|FlowControl|Switch|SwitchonE_GamingStat (Variables|Default|GetGamingMode)
    (:NewEnumerator0
      (Variables|Default|SetGamingMode "NewEnumerator1")
      (Default|CallEDPause)
      (Utilities|IsValid (Variables|Default|GetPauseMenu)
        (:Is%20Valid
          (Widget|SetVisibility (Variables|Default|GetPauseMenu) "Visible"))
        (:Is%20Not%20Valid
          (bind _returnvalue (UserInterface|CreateWidget "/Game/ATI/Entity/Player/HUD/Pause.Pause_C"))
          (bind _output_get (Variables|Default|SetPauseMenu _returnvalue))
          (UserInterface|Viewport|AddtoViewport _output_get 1))))
    (:NewEnumerator1
      (Variables|Default|SetGamingMode "NewEnumerator0")
      (Default|CallEDPause)
      (Widget|SetVisibility (Variables|Default|GetPauseMenu) "Hidden"))))

(event Custom|ResetLvl
  (for _array_element (Variables|Default|GetSubLvlReset)
    (Class|GameplayStatics|UnloadStreamLevelbySoftObjectPtr _array_element false))
  (Utilities|FlowControl|Delay 0.1)
  (for _array_element_2 (Variables|Default|GetSubLvlReset)
    (Class|GameplayStatics|LoadStreamLevelbySoftObjectPtr _array_element_2 true false)))

(event Custom|Exit)

(fn ConstructionScript)

(fn AddSubLvlReset
  (params (SubLvlReset :type World%20Soft%20Object%20Reference))
  (Utilities|Array|AddUnique (Variables|Default|GetSubLvlReset) SubLvlReset))

(fn SetSubLvlReset
  (params (SubLvlReset :type Array%20of%20World%20Soft%20Object%20References))
  (Variables|Default|SetSubLvlReset SubLvlReset))

(fn RemoveSubLvlReset
  (params (SubLvlReset :type World%20Soft%20Object%20Reference))
  (Utilities|Array|RemoveItem (Variables|Default|GetSubLvlReset) SubLvlReset))

(fn ClearSubLvlReset
  (Utilities|Array|Clear (Variables|Default|GetSubLvlReset)))